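; BP_Lever_DOORLINK is a lever that controls a linked door when the player interacts with it.
; The PlayerInteracted event copies the lever's Active state into the Door's IsDoorOpen flag, then calls UpdateDoor on that door to apply it.
; It also prints a debug "Hello" string; the construction script only calls its parent, and the other event stubs are disabled.
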(event `self.PlayerInteracted`
  (bind _door (`self.Door`))
  (set `/Game/Blueprints/BP_Door.IsDoorOpen` (`self.Active`) _door)
  (`/Game/Blueprints/BP_Door.UpdateDoor` _door)
  (`KismetSystemLibrary.PrintString` "Hello"))

(fn `UserConstructionScript`
  (`parent.UserConstructionScript`))