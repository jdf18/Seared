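; BP_Checkpoint is a level-exit checkpoint actor that advances the game to the next level when the player reaches it.
; On BeginPlay it caches the BP_GameInstance.
; An overlap on its Ere component by an actor tagged "Player" calls ProgressToNextLevel on that instance.
; A DoOnce gate, reset after a short delay, guards against repeated triggers from rapid overlaps.
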(event `self.ReceiveBeginPlay`
  (bind _asbp_game_instance (cast `/Game/Blueprints/BP_GameInstance` (`GameplayStatics.GetGameInstance`))))

(event `self.ere.OnComponentBeginOverlap`
  (params (OverlappedComponent :type "PrimitiveComponent Object Reference") (OtherActor :type "Actor Object Reference") (OtherComp :type "PrimitiveComponent Object Reference") (OtherBodyIndex :type Integer) (bFromSweep :type Boolean) (SweepResult :type "HitResult Structure (by ref)"))
  (if (!= (`KismetArrayLibrary.Array_Find` (`Actor.Tags` OtherActor) "Player") -1)
    (`/Engine/EditorBlueprintResources/StandardMacros.DoOnce` false :!label _label
      (:`Completed`
        (`self.GoToNextLevel` (stale `self.ReceiveBeginPlay` _asbp_game_instance))
        (`KismetSystemLibrary.Delay` 0.2)
        (goto _label :!via `Reset`)))))

(fn `GoToNextLevel`
  (params (GameInstance :type "/Game/Blueprints/BP_GameInstance Object Reference"))
  (`/Game/Blueprints/BP_GameInstance.ProgressToNextLevel` GameInstance))

(fn `UserConstructionScript`)