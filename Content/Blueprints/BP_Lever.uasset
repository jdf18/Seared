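; BP_Lever is a toggleable lever that shows an image prompt widget while a player overlaps its box.
; CallPlayerTryInteract fires the interact event, which checks for an overlapping player, flips Active and swaps the on/off sprite.
; A DoOnce reset after a short delay acts as a cooldown between toggles.
; PlayerInteracted runs on each toggle but only prints a debug message here.
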(event `self.ReceiveBeginPlay`
  (bind _asw_image_prompt (cast `/Game/Blueprints/W_ImagePrompt` (`WidgetComponent.GetUserWidgetObject` (`self.WidgetLever`))))
  (`/Game/Blueprints/W_ImagePrompt.Set Texture` _asw_image_prompt "/Game/Assets/Sprites/UI/E_Popup.E_Popup"))

(event `playerTryInteract`
  ;[1 1 1] If there is a player in range
  (if (!= (`KismetArrayLibrary.Array_Length` (`PrimitiveComponent.GetOverlappingActors` (`self.Box`) "/Game/Blueprints/BP_PlayerBase.BP_PlayerBase_C")) 0)
    ;[1 1 1] Lever interaction call + cooldown
    (`/Engine/EditorBlueprintResources/StandardMacros.DoOnce` false :!label _label
      (:`Completed`
        (bind _output_get (set `self.Active` (not (stale _output_get))))
        (`|ExecutionSequence`
          (:`then_0`
            ;[1 1 1] Set correct lever image
            (`PaperSpriteComponent.SetSprite` (`self.Sprite`) (select `bool` _output_get :`false` "/Game/Assets/Sprites/Activatables/toggleleveroff_Sprite.toggleleveroff_Sprite" :`true` "/Game/Assets/Sprites/Activatables/toggleleveron_Sprite.toggleleveron_Sprite" :!type "PaperSprite Object Reference")))
          (:`then_1`
            (`self.PlayerInteracted`))
          (:`then_2`
            (`KismetSystemLibrary.Delay` 0.5)
            (goto _label :!via `Reset`)))))))

(event `PlayerInteracted`
  ;[1 1 1] Is there a player in range
  (`KismetSystemLibrary.PrintString` "Player Interacted with Lever" true true (struct :`G` 0.66 :`B` 1.0 :`A` 1.0) 0.0))

(event `self.Box.OnComponentBeginOverlap`
  (params (OverlappedComponent :type "PrimitiveComponent Object Reference") (OtherActor :type "Actor Object Reference") (OtherComp :type "PrimitiveComponent Object Reference") (OtherBodyIndex :type Integer) (bFromSweep :type Boolean) (SweepResult :type "HitResult Structure (by ref)"))
  (cast `/Game/Blueprints/BP_PlayerBase` OtherActor)
  (`SceneComponent.SetHiddenInGame` (`self.WidgetLever`) false false))

(event `self.Box.OnComponentEndOverlap`
  (params (OverlappedComponent :type "PrimitiveComponent Object Reference") (OtherActor :type "Actor Object Reference") (OtherComp :type "PrimitiveComponent Object Reference") (OtherBodyIndex :type Integer))
  (cast `/Game/Blueprints/BP_PlayerBase` OtherActor)
  (`SceneComponent.SetHiddenInGame` (`self.WidgetLever`) true false))

(fn `CallPlayerTryInteract`
  ;[1 1 1] Function to call event DO NOT REMOVE
  (`self.playerTryInteract`))

(fn `UserConstructionScript`)