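; BP_Popup is a world prompt actor that shows a text widget while a player is inside its trigger box.
; On BeginPlay it passes its TextIn value to the W_Prompt widget hosted by TextWidget.
; Box overlap begin and end events unhide and hide TextWidget, responding only to BP_PlayerBase actors.
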(event `self.ReceiveBeginPlay`
  (bind _asw_prompt (cast `/Game/Blueprints/W_Prompt` (`WidgetComponent.GetUserWidgetObject` (`self.TextWidget`))))
  (`/Game/Blueprints/W_Prompt.SetPromptText` _asw_prompt (`self.Text In`)))

(event `self.Box.OnComponentBeginOverlap`
  (params (OverlappedComponent :type "PrimitiveComponent Object Reference") (OtherActor :type "Actor Object Reference") (OtherComp :type "PrimitiveComponent Object Reference") (OtherBodyIndex :type Integer) (bFromSweep :type Boolean) (SweepResult :type "HitResult Structure (by ref)"))
  (cast `/Game/Blueprints/BP_PlayerBase` OtherActor)
  (`SceneComponent.SetHiddenInGame` (`self.TextWidget`) false false))

(event `self.Box.OnComponentEndOverlap`
  (params (OverlappedComponent :type "PrimitiveComponent Object Reference") (OtherActor :type "Actor Object Reference") (OtherComp :type "PrimitiveComponent Object Reference") (OtherBodyIndex :type Integer))
  (cast `/Game/Blueprints/BP_PlayerBase` OtherActor)
  (`SceneComponent.SetHiddenInGame` (`self.TextWidget`) true false))

(fn `UserConstructionScript`)