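; BP_Crate1 is a crate actor tied to a spline that shows an interaction prompt when a player is near.
; On BeginPlay it sets the E_Popup image on its prompt widget and snaps to the start of the spline.
; InteractionBox overlaps with BP_PlayerBase show and hide the widget.
; Helper functions return the normalized spline tangent nearest a position and set the root's world location, with no movement logic in this graph.
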(event `self.ReceiveBeginPlay`
  (`|ExecutionSequence`
    (:`then_0`
      (bind _asw_image_prompt (cast `/Game/Blueprints/W_ImagePrompt` (`WidgetComponent.GetUserWidgetObject` (`self.Widget`))))
      (`/Game/Blueprints/W_ImagePrompt.Set Texture` _asw_image_prompt "/Game/Assets/Sprites/UI/E_Popup.E_Popup"))
    (:`then_1`
      (`self.K2_SetActorLocation` (`SplineComponent.GetLocationAtTime` (`self.Spline`) 0.0 "World" false)))))

(event `self.InteractionBox.OnComponentBeginOverlap`
  (params (OverlappedComponent :type "PrimitiveComponent Object Reference") (OtherActor :type "Actor Object Reference") (OtherComp :type "PrimitiveComponent Object Reference") (OtherBodyIndex :type Integer) (bFromSweep :type Boolean) (SweepResult :type "HitResult Structure (by ref)"))
  (cast `/Game/Blueprints/BP_PlayerBase` OtherActor)
  (`SceneComponent.SetHiddenInGame` (`self.Widget`) false false))

(event `self.InteractionBox.OnComponentEndOverlap`
  (params (OverlappedComponent :type "PrimitiveComponent Object Reference") (OtherActor :type "Actor Object Reference") (OtherComp :type "PrimitiveComponent Object Reference") (OtherBodyIndex :type Integer))
  (cast `/Game/Blueprints/BP_PlayerBase` OtherActor)
  (`SceneComponent.SetHiddenInGame` (`self.Widget`) true false))

(fn `GetTangentToPos`
  (params (Position :type "Vector Structure"))
  (returns (Direction :type "Vector Structure"))
  (locals (selfs :type "Pawn Object Reference"))
  (return (`KismetMathLibrary.Normal` (`SplineComponent.FindTangentClosestToWorldLocation` (`self.Spline`) Position "World"))))

(fn `SetPosition`
  (params (Location :type "Vector Structure"))
  (`SceneComponent.K2_SetWorldLocation` (`self.RootComponent`) Location false false))

(fn `UserConstructionScript`)