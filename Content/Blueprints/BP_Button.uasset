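; BP_Button is an interactable button with a cooldown that swaps between active and inactive sprites.
; playerTryInteract debug-prints whether a BP_PlayerBase overlaps its Box, and if so passes a DoOnce gate to show the active sprite.
; Both Sequence branches call PlayerInteracted, which only prints a message, and share one ButtonCooldown delay that restores the inactive sprite and resets the gate.
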(event `playerTryInteract`
  (bind _sprite (`self.Sprite`))
  (bind _returnvalue (!= (`KismetArrayLibrary.Array_Length` (`PrimitiveComponent.GetOverlappingActors` (`self.Box`) "/Game/Blueprints/BP_PlayerBase.BP_PlayerBase_C")) 0))
  (`KismetSystemLibrary.PrintString` (`KismetStringLibrary.Conv_BoolToString` _returnvalue))
  (if _returnvalue
    (`/Engine/EditorBlueprintResources/StandardMacros.DoOnce` false :!label _label
      (:`Completed`
        (`|ExecutionSequence`
          (:`then_0`
            (`PaperSpriteComponent.SetSprite` _sprite "/Game/Assets/Sprites/Buttons/SpriteButtonActive.SpriteButtonActive"))
          (:`then_1`
            _))
        (`self.PlayerInteracted`)
        (`KismetSystemLibrary.Delay` (`self.ButtonCooldown`))
        (`PaperSpriteComponent.SetSprite` _sprite "/Game/Assets/Sprites/Buttons/SpriteButtonInactive.SpriteButtonInactive")
        (goto _label :!via `Reset`)))))

(event `PlayerInteracted`
  (`KismetSystemLibrary.PrintString` "Player Interacted with button"))

(fn `CallPlayerTryInteract`
  (`self.playerTryInteract`))

(fn `UserConstructionScript`)