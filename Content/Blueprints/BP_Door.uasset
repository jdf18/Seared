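; BP_Door is a 2D Paper2D door that switches between open and closed states.
; OpenDoor and CloseDoor set the IsDoorOpen flag and call UpdateDoor, which swaps the sprite and disables or restores the Box collision to match.
; The door starts closed on BeginPlay, and nothing in this Blueprint calls OpenDoor.
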(event `self.ReceiveBeginPlay`
  (`self.CloseDoor`))

(fn `CloseDoor`
  (set `self.IsDoorOpen` false)
  (`self.UpdateDoor`))

(fn `OpenDoor`
  (set `self.IsDoorOpen` true)
  (`self.UpdateDoor`))

(fn `UpdateDoor`
  (bind _isdooropen (`self.IsDoorOpen`))
  (`PaperSpriteComponent.SetSprite` (`self.PaperSprite`) (select `bool` _isdooropen :`false` "/Game/Assets/Sprites/Activatables/doorclosed_Sprite_0.doorclosed_Sprite_0" :`true` "/Game/Assets/Sprites/Activatables/dooropen_Sprite_0.dooropen_Sprite_0" :!type "PaperSprite Object Reference"))
  (`PrimitiveComponent.SetCollisionEnabled` (`self.Box`) (select `bool` _isdooropen :`false` "QueryAndPhysics" :`true` "NoCollision" :!type "ECollisionEnabled Enum")))

(fn `UserConstructionScript`
  (set `self.IsDoorOpen` false))